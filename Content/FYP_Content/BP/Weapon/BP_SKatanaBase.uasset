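; Katana weapon base Blueprint that sets the normal attack montage and deals melee damage through swept blade traces.
; While attack detection runs, a looping timer sphere-traces from each current tracking point to its previous position, with debug drawing on.
; Hit actors are recorded so each takes damage once per detection window; the owner is ignored.
; BPGetTrackingPoint builds evenly spaced points from the RangeStart socket toward RangeEnd.
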(event `self.ReceiveBeginPlay`
  (set `self.AttackMontage` "/Game/FYP_Content/Animation/Retargeted/Equip_Weapon/AM_Weapon_Normal_Attack.AM_Weapon_Normal_Attack"))

(event `self.ReceiveTick`
  (params (DeltaSeconds :type "Float (single-precision)")))

(event `AttackDetection_BP`
  (`|ExecutionSequence`
    (:`then_0`
      (set `self.Prev_TrackingPoints_0` (`self.GetTrackingPoints`))
      (`BlueprintSetLibrary.Set_Clear` (`self.HitActors_0`)))
    (:`then_1`
      (bind _returnvalue (`KismetSystemLibrary.K2_SetTimerDelegate` (delegate `Tracking`) 0.01 true))
      (set `self.TrackingTimerHandle` _returnvalue))))

(event `StopAttackDetection_BP`
  (bind _trackingtimerhandle (`self.TrackingTimerHandle`))
  (if (`KismetSystemLibrary.K2_IsValidTimerHandle` _trackingtimerhandle)
    (`KismetSystemLibrary.K2_ClearAndInvalidateTimerHandle` _trackingtimerhandle)))

(event `Tracking`
  (bind _output_get (set `self.Cur_TrackingPoints` (`self.GetTrackingPoints`)))
  (for (_array_element _array_index) _output_get
    (bind (_outhit _returnvalue) (`KismetSystemLibrary.SphereTraceSingle` _array_element (`|GetArrayItem` (`self.Prev_TrackingPoints_0`) _array_index) 10.0 "TraceTypeQuery1" false (`|MakeArray` (`self.GetOwner`)) "ForDuration"))
    (if _returnvalue
      (bind _result (`BlueprintSetLibrary.Set_ToArray` (`self.HitActors_0`)))
      (bind (_bblockinghit _binitialoverlap _time _distance _location _impactpoint _normal _impactnormal _physmat _hitactor) (`GameplayStatics.BreakHitResult` _outhit))
      (if (== (`KismetArrayLibrary.Array_Find` _result _hitactor) -1)
        (`GameplayStatics.ApplyDamage` _hitactor (`self.DamageValue`) (`self.GetInstigatorController`) self "/Script/Engine.DamageType")
        (`BlueprintSetLibrary.Set_Add` (`self.HitActors_0`) _hitactor))))
  (`KismetArrayLibrary.Array_Clear` (`self.Prev_TrackingPoints_0`))
  (set `self.Prev_TrackingPoints_0` (`self.Cur_TrackingPoints`)))

(fn `BP_GetTrackingPoint`
  (returns (NewParam :type "Array of Vector Structure"))
  (locals (Points :type "Array of Vector Structure"))
  (bind _katana (`self.Katana`))
  (bind _returnvalue (`SceneComponent.GetSocketLocation` _katana "RangeStart"))
  (for _index (range 5)
    (`KismetArrayLibrary.Array_Add` (`local.Points`) (+ _returnvalue (* _index (* (`KismetMathLibrary.GetForwardVector` (`KismetMathLibrary.FindLookAtRotation` _returnvalue (`SceneComponent.GetSocketLocation` _katana "RangeEnd"))) 25)))))
  (return (`local.Points`)))

(fn `UserConstructionScript`)