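; BP_ContainerComponent is an inventory component that records collected items and their counts in an Items map.
; CollectItem adds a new item with a count of one; for an existing item, it writes the incremented count under the "None" key instead of that item's key.
; After each collection, it prints every key in the map to the screen.
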(event `CollectItem`
  (params (Item :type Name))
  (bind _items (`self.Items`))
  (bind (_value _returnvalue) (`BlueprintMapLibrary.Map_Find` _items Item))
  (if _returnvalue
    (`BlueprintMapLibrary.Map_Add` _items "None" (+ _value 1))
    (else
      (`BlueprintMapLibrary.Map_Add` _items Item 1)))
  (bind _keys (`BlueprintMapLibrary.Map_Keys` (`self.Items`)))
  (for _array_element _keys
    (`KismetSystemLibrary.PrintString` (`KismetStringLibrary.Conv_NameToString` _array_element))))