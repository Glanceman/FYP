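; BP_SDoorBase is a door actor that opens when a BP_SCharacter overlaps it, optionally requiring a key.
; Unless TriggerKeyName is "Any", the character's item container must hold that name, otherwise a "No Required Key" message prints.
; TriggertoUnlock and TriggertoLock events call Open and Close directly, bypassing the key check.
; Open and Close are called here but defined outside these graphs.
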(event `self.ReceiveActorBeginOverlap`
  (params (OtherActor :type "Actor Object Reference"))
  (bind _asbp_scharacter (cast `/Game/FYP_Content/BP/Character/Hero/BP_SCharacter` OtherActor))
  (if (!= (`self.TriggerKeyName`) "Any")
    (if (`BlueprintMapLibrary.Map_Contains` (`SItemContainerComponent.ItemsName` (`SCharacter.SItemContainerComponent` _asbp_scharacter)) (`self.TriggerKeyName`))
      (`self.Open` 0.0)
      (else
        (`KismetSystemLibrary.PrintString` "No Required Key" true true (struct :`G` 0.66 :`B` 1.0 :`A` 1.0) 10.0)))
    (else
      (`self.Open` 0.0))))

(event `SPuzzleTriggerInterface.TriggerToUnlock`
  (`self.Open` 0.0))

(event `SPuzzleTriggerInterface.TriggerToLock`
  (`self.Close` 0.0))

(fn `UserConstructionScript`)