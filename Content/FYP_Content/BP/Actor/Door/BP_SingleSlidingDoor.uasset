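; BP_SingleSlidingDoor is a door actor with a single sliding panel that opens and closes along its local X axis.
; BeginPlay stores the Point component's relative X and derives the open position by subtracting SlidingRange.
; Open plays a timeline that lerps Point between those two positions, and Close reverses the same timeline.
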(event `self.ReceiveBeginPlay`
  (bind _relativelocation_x (`KismetMathLibrary.BreakVector` (`SceneComponent.RelativeLocation` (`self.Point`))))
  (bind _output_get (set `self.InitLocation` _relativelocation_x))
  (set `self.TargetLocation` (- _output_get (`self.SlidingRange`))))

(event `self.Open`
  (params (DeltaTime :type "Float (single-precision)"))
  (bind (_direction _alpha) (`Timeline|Timeline` :!label _label)
    (:`Update`
      (`SceneComponent.K2_SetRelativeLocation` (`self.Point`) (`KismetMathLibrary.MakeVector` (`KismetMathLibrary.Lerp` (`self.InitLocation`) (`self.TargetLocation`) _alpha)) false false))))

(event `self.Close`
  (params (DeltaTime :type "Float (single-precision)"))
  (goto _label :!via `Reverse`))

(fn `UserConstructionScript`)