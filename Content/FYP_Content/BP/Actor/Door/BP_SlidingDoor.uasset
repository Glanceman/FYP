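; BP_SlidingDoor is a two-panel sliding door actor with Open and Close events and a looping stone-scrape sound.
; BeginPlay derives the target X from the Right panel's position and MovingRange.
; One timeline, played to open and reversed to close, lerps the Right panel's X from InitLocation and mirrors it onto Left.
; The scrape loop respawns when no live audio component exists and stops when the timeline finishes.
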(event `self.ReceiveBeginPlay`
  (bind _relativelocation_x (`KismetMathLibrary.BreakVector` (`SceneComponent.RelativeLocation` (`self.Right`))))
  (set `self.RightTargetLocation` (- _relativelocation_x (`self.MovingRange`))))

(event `self.ReceiveActorEndOverlap`
  (params (OtherActor :type "Actor Object Reference")))

(event `self.Open`
  (params (DeltaTime :type "Float (single-precision)"))
  (bind _audiocomponent (`self.AudioComponent`))
  (`/Engine/EditorBlueprintResources/StandardMacros.IsValid` _audiocomponent
    (:`Is Valid`
      (if (`ActorComponent.IsBeingDestroyed` _audiocomponent)
        (bind _returnvalue (`GameplayStatics.SpawnSoundAtLocation` "/Game/FYP_Content/BP/Actor/Door/Sound/StoneScrapeLoop_Cue.StoneScrapeLoop_Cue" (`self.K2_GetActorLocation`) (struct) 1.0 1.0 0.0 null null :!label _label))
        (set `self.AudioComponent` _returnvalue)
        (bind (_direction _alpha) (`Timeline|Timeline` :!label _label_2)
          (:`Update`
            (`|ExecutionSequence`
              (:`then_0`
                (bind _returnvalue_2 (`KismetMathLibrary.Lerp` (`self.InitLocation`) (`self.RightTargetLocation`) _alpha))
                (`SceneComponent.K2_SetRelativeLocation` (`self.Right`) (`KismetMathLibrary.MakeVector` _returnvalue_2) false false))
              (:`then_1`
                (`SceneComponent.K2_SetRelativeLocation` (`self.Left`) (`KismetMathLibrary.MakeVector` (* _returnvalue_2 -1.0)) false false))))
          (:`Finished`
            (`AudioComponent.Stop` (`self.AudioComponent`))))
        (else
          (goto _label_2))))
    (:`Is Not Valid`
      (goto _label))))

(event `self.Close`
  (params (DeltaTime :type "Float (single-precision)"))
  (bind _audiocomponent (`self.AudioComponent`))
  (`/Engine/EditorBlueprintResources/StandardMacros.IsValid` _audiocomponent
    (:`Is Valid`
      (if (`ActorComponent.IsBeingDestroyed` _audiocomponent)
        _
        (else
          (goto _label_2 :!via `Reverse`))))
    (:`Is Not Valid`
      _))
  (bind _returnvalue (`GameplayStatics.SpawnSoundAtLocation` "/Game/FYP_Content/BP/Actor/Door/Sound/StoneScrapeLoop_Cue.StoneScrapeLoop_Cue" (`self.K2_GetActorLocation`) (struct) 1.0 1.0 0.0 null null))
  (set `self.AudioComponent` _returnvalue)
  (goto _label_2 :!via `Reverse`))

(fn `UserConstructionScript`)