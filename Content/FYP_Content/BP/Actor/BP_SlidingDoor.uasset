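; BP_SlidingDoor is a two-panel sliding door actor that closes when an SCharacterBase stops overlapping it.
; BeginPlay derives the target X from the Right panel's relative position minus MovingRange.
; Open plays a timeline that lerps Right from InitLocation to that target and mirrors Left by negating the value, and Close reverses it.
; Nothing in this graph calls Open.
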(event `self.ReceiveBeginPlay`
  (bind _relativelocation_x (`KismetMathLibrary.BreakVector` (`SceneComponent.RelativeLocation` (`self.Right`))))
  (set `self.RightTargetLocation` (- _relativelocation_x (`self.MovingRange`))))

(event `self.ReceiveActorEndOverlap`
  (params (OtherActor :type "Actor Object Reference"))
  (cast `SCharacterBase` OtherActor)
  (`self.Close` 0.0))

(event `self.Open`
  (params (DeltaTime :type "Float (single-precision)"))
  (bind (_direction _alpha) (`Timeline|Timeline` :!label _label)
    (:`Update`
      (`|ExecutionSequence`
        (:`then_0`
          (bind _returnvalue (`KismetMathLibrary.Lerp` (`self.InitLocation`) (`self.RightTargetLocation`) _alpha))
          (`SceneComponent.K2_SetRelativeLocation` (`self.Right`) (`KismetMathLibrary.MakeVector` _returnvalue) false false))
        (:`then_1`
          (`SceneComponent.K2_SetRelativeLocation` (`self.Left`) (`KismetMathLibrary.MakeVector` (* _returnvalue -1.0)) false false))))))

(event `self.Close`
  (params (DeltaTime :type "Float (single-precision)"))
  (goto _label :!via `Reverse`))

(fn `UserConstructionScript`)