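; A kill/respawn volume actor that catches anything falling or wandering out of bounds.
; On overlap, a BP_SCharacter is teleported back to its LastOnGroundLocation with its movement velocity zeroed.
; BP_SBladeBase actors are left untouched, and any other overlapping actor is destroyed.
; The construction script sizes the trigger Box from the Size variable.
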(event `self.ReceiveActorBeginOverlap`
  (params (OtherActor :type "Actor Object Reference"))
  (bind _asbp_scharacter (cast `/Game/FYP_Content/BP/Character/Hero/BP_SCharacter` OtherActor)
    (:`then`
      (`self.K2_SetActorLocation` _asbp_scharacter (`SCharacterBase.LastOnGroundLocation` _asbp_scharacter) false true)
      (set `MovementComponent.Velocity` (0.0 0.0 0.0) (`Pawn.GetMovementComponent` _asbp_scharacter)))
    (:`CastFailed`
      (cast `/Game/FYP_Content/BP/Actor/Weapon/BP_SBladeBase` OtherActor
        (:`CastFailed`
          (`self.K2_DestroyActor` OtherActor))))))

(fn `UserConstructionScript`
  (`BoxComponent.SetBoxExtent` (`self.Box`) (`self.Size`) true))