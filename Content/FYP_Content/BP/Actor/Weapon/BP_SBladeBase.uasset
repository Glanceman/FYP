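; Base actor for a throwable blade weapon that the player can throw, stick into what it hits and recall to the hand.
; Throwing uses projectile and rotating movement while a timeline line-traces along velocity to stop, orient and attach the blade.
; Recall launches an attached character or physics object toward the player, then detaches.
; A distance-scaled timeline curves the spinning blade back to the hand socket, sphere-tracing for damage and calling Caught.
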(event `self.ReceiveTick`
  (params (DeltaSeconds :type "Float (single-precision)")))

(event `self.ReceiveBeginPlay`
  (bind (_returnvalue_roll _returnvalue_pitch _returnvalue_yaw) (`KismetMathLibrary.BreakRotator` (`self.K2_GetActorRotation`)))
  (bind (_offsetrotation_roll _offsetrotation_pitch _offsetrotation_yaw) (`KismetMathLibrary.BreakRotator` (`self.OffsetRotation`)))
  (bind _asscharacter (cast `SCharacter` (`GameplayStatics.GetPlayerCharacter` 0)))
  (set `self.PlayerRef` _asscharacter)
  ;[1 1 1] Match orientation with shooting direction when spawn
  (`self.K2_SetActorRotation` (`KismetMathLibrary.MakeRotator` (+ _returnvalue_roll _offsetrotation_roll) (+ _returnvalue_pitch _offsetrotation_pitch) (+ _returnvalue_yaw _offsetrotation_yaw))))

(event `ShootInDirection`
  (params (DirVector :type "Vector Structure"))
  (bind _projectilemovementcomponent (`self.ProjectileMovementComponent`))
  (bind (_returnvalue_roll _returnvalue_pitch _returnvalue_yaw) (`KismetMathLibrary.BreakRotator` (`KismetMathLibrary.FindLookAtRotation` (`self.K2_GetActorLocation`) (`self.ImpactPoint`))))
  (`|ExecutionSequence`
    (:`then_0`
      ;[1 1 1] Init
      (set `MovementComponent.Velocity` (* DirVector (`ProjectileMovementComponent.InitialSpeed` _projectilemovementcomponent)) _projectilemovementcomponent)
      (`ActorComponent.Activate` (`self.ProjectileMovementComponent`) false)
      (`ActorComponent.Activate` (`self.RotatingMovement`) false)
      (set `ProjectileMovementComponent.ProjectileGravityScale` 1.0 (`self.ProjectileMovementComponent`)))
    (:`then_1`
      (`Timeline|Throw_TimeLine` :!via `PlayFromStart`
        (:`Update`
          (if (!= (`self.K2_GetActorLocation` self) (`SceneComponent.GetSocketLocation` (`Character.Mesh` (`self.PlayerRef`)) "DEF-weapon_R"))
            (bind _outhit (`KismetSystemLibrary.LineTraceSingle` :`Start` (`self.K2_GetActorLocation`) :`End` (+ (`self.K2_GetActorLocation`) (* (`KismetMathLibrary.Normal` (`self.GetVelocity`)) (`self.TraceDist`))) :`TraceChannel` "TraceTypeQuery1" :`DrawDebugType` "ForDuration"))
            (bind (_bblockinghit _binitialoverlap _time _distance _location _impactpoint _normal _impactnormal _physmat _hitactor) (`GameplayStatics.BreakHitResult` _outhit))
            (if _bblockinghit
              (`|ExecutionSequence`
                (:`then_0`
                  ;[1 1 1] compute rotation when get hit
                  (set `self.ImpactNormal` _impactnormal)
                  (set `self.ImpactPoint` _impactpoint)
                  (`MovementComponent.StopMovementImmediately` (`self.ProjectileMovementComponent`))
                  (`ActorComponent.Deactivate` (`self.ProjectileMovementComponent`))
                  (`ActorComponent.Deactivate` (`self.RotatingMovement`))
                  (`self.K2_SetActorRotation` (`KismetMathLibrary.MakeRotator` _returnvalue_roll _returnvalue_pitch _returnvalue_yaw))
                  (`SceneComponent.K2_SetRelativeRotation` (`self.blade`) (`self.OffsetRotation`) false false)
                  (`KismetSystemLibrary.PrintString` "Hit")
                  (`ActorComponent.Deactivate` (`self.Throw_TimeLine`)))
                (:`then_1`
                  (`self.K2_AttachToActor` self _hitactor "None" "KeepWorld" "KeepWorld" "KeepWorld" true))))))))))

(event `Recall_Event`
  (bind _returnvalue (`self.K2_GetActorLocation`))
  (bind _starttransformation_location (`KismetMathLibrary.BreakTransform` (`self.StartTransformation`)))
  (bind (_offsetrotation_roll _offsetrotation_pitch _offsetrotation_yaw) (`KismetMathLibrary.BreakRotator` (`self.OffsetRotation`)))
  (bind _starttransformation_location_2 (`KismetMathLibrary.BreakTransform` (`self.StartTransformation`)))
  (bind _recalldestination_location (`KismetMathLibrary.BreakTransform` (`self.RecallDestination`)))
  (bind (_returnvalue_roll _returnvalue_pitch _returnvalue_yaw) (`KismetMathLibrary.BreakRotator` (`KismetMathLibrary.FindLookAtRotation` (`self.CurrentLocation`) (`self.lastTickLocation`))))
  (bind _camera (`SCharacter.Camera` (`self.PlayerRef`)))
  (bind _returnvalue_2 (`self.GetComponentByClass` (`self.GetAttachParentActor` self) "/Script/Engine.PrimitiveComponent"))
  (bind _returnvalue_3 (+ (* (`KismetMathLibrary.Normal` (- (`self.K2_GetActorLocation` (`self.PlayerRef`)) (`self.K2_GetActorLocation`))) 1500.0) (0.0 0.0 250.0)))
  (`|ExecutionSequence`
    (:`then_0`
      ;[1 1 1] Init
      (`ActorComponent.Deactivate` (`self.Throw_TimeLine`))
      (`ActorComponent.Deactivate` (`self.ProjectileMovementComponent`))
      (`ActorComponent.Deactivate` (`self.RotatingMovement`))
      (set `self.StartTransformation` (`self.GetTransform`))
      (set `self.RecallDist` (`KismetMathLibrary.VSize` (- _starttransformation_location (`SceneComponent.GetSocketLocation` (`Character.Mesh` (`self.PlayerRef`)) "DEF-weapon_R"))))
      (set `self.RecallPlayRate` (`KismetMathLibrary.FClamp` (/ (`self.RefRecallDist`) (`self.RecallDist`)) 0.5 8.0))
      (set `self.lastTickLocation` _returnvalue)
      (set `self.CurrentLocation` _returnvalue))
    (:`then_1`
      (`|ExecutionSequence`
        (:`then_0`
          ;[1 1 1] pull target
          (if (`KismetSystemLibrary.IsValid` (`self.GetAttachParentActor` self))
            (bind _ascharacter (cast `Character` (`self.GetAttachParentActor` self))
              (:`then`
                (if (`KismetSystemLibrary.IsValid` _ascharacter)
                  (`Character.LaunchCharacter` _ascharacter _returnvalue_3 false false)))
              (:`CastFailed`
                (if (and (`KismetSystemLibrary.IsValid` _returnvalue_2) (`SceneComponent.IsSimulatingPhysics` _returnvalue_2 "None"))
                  (`PrimitiveComponent.AddImpulse` _returnvalue_2 _returnvalue_3 "None" true))))))
        (:`then_1`
          (`self.K2_DetachFromActor` self "KeepWorld" "KeepWorld" "KeepWorld")
          (`TimelineComponent.SetPlayRate` (`self.Recall_TimeLine`) (`self.RecallPlayRate`))
          (set `self.NumberOfSpin` (/ (* (/ 1.0 (`self.RecallPlayRate`)) (`TimelineComponent.GetTimelineLength` (`self.Recall_TimeLine`))) (`self.SpinRate`)))
          (bind (_direction _locationalpha _offsetalpha _spinningalpha _rotationtosocket) (`Timeline|Recall_TimeLine` :!via `PlayFromStart`)
            (:`Update`
              ;[1 1 1] Updated
              (`|ExecutionSequence`
                (:`then_0`
                  (set `self.RecallDestination` (`SceneComponent.GetSocketTransform` (`Character.Mesh` (`self.PlayerRef`)) "DEF-weapon_R" "RTS_World"))
                  (set `self.lastTickLocation` (`self.K2_GetActorLocation`))
                  (bind _output_get (set `self.CurrentLocation` (`KismetMathLibrary.VLerp` _starttransformation_location_2 (+ (* (`KismetMathLibrary.Normal` (+ (`SceneComponent.GetUpVector` _camera) (* (`SceneComponent.GetRightVector` _camera) -1.0))) (* (/ (`self.RecallDist`) 2.0) _offsetalpha)) _recalldestination_location) _locationalpha)))
                  (`self.K2_SetActorLocation` _output_get)
                  (`self.K2_SetActorRotation` (`KismetMathLibrary.RLerp` (`KismetMathLibrary.MakeRotator` _returnvalue_roll _returnvalue_pitch (+ _returnvalue_yaw _offsetrotation_yaw)) (`SceneComponent.GetSocketRotation` (`Character.Mesh` (`self.PlayerRef`)) "DEF-weapon_R") _rotationtosocket true))
                  (`SceneComponent.K2_SetRelativeRotation` (`self.blade`) (`KismetMathLibrary.MakeRotator` (* (`KismetMathLibrary.MapRangeClamped` _spinningalpha 0.0 1.0 0.0 (`self.NumberOfSpin`)) -360.0) _returnvalue_pitch) false false))
                (:`then_1`
                  (bind (_outhit _returnvalue_4) (`KismetSystemLibrary.SphereTraceSingle` (`self.lastTickLocation`) (`self.CurrentLocation`) 25.0 "TraceTypeQuery1" false (`|MakeArray` (`self.PlayerRef`) :!type "Actor Object Reference") "ForDuration"))
                  (if _returnvalue_4
                    (`GameplayStatics.ApplyDamage` (`.HitActor` (`GameplayStatics.BreakHitResult` _outhit)) 1.0 null self "/Script/Engine.DamageType")))))
            (:`Finished`
              ;[1 1 1] Finish
              (bind _asbp_scharacter (cast `/Game/FYP_Content/BP/Character/Hero/BP_SCharacter` (`self.PlayerRef`)))
              (`SceneComponent.K2_SetRelativeRotation` (`self.blade`) (`self.OffsetRotation`) false false)
              (`/Game/FYP_Content/BP/Character/Hero/BP_SCharacter.Caught` _asbp_scharacter))))))))

(fn `UserConstructionScript`)