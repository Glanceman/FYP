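; BP_BlockToAnimation is a one-shot trigger actor that shows the WB_StartText widget and plays its animation on overlap.
; The first overlap sets Triggered, then resolves the overlapping Pawn's PlayerController, adds the widget to the viewport and calls PlayAnim with that controller.
; Triggered is set before the casts, so a first overlap by anything other than a player-controlled Pawn uses up the trigger without showing the widget.
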(event `self.ReceiveActorBeginOverlap`
  (params (OtherActor :type "Actor Object Reference"))
  (if (== (`self.bTriggered`) false)
    (set `self.bTriggered` true)
    (bind _aspawn (cast `Pawn` OtherActor))
    (bind _asplayer_controller (cast `PlayerController` (`Pawn.GetController` _aspawn)))
    (bind _returnvalue (`|CreateWidget` "/Game/FYP_Content/BP/UI/WB_StartText.WB_StartText_C" _asplayer_controller))
    (`UserWidget.AddToViewport` _returnvalue 0)
    (`/Game/FYP_Content/BP/UI/WB_StartText.PlayAnim` _returnvalue _asplayer_controller)))

(fn `UserConstructionScript`
  (`parent.UserConstructionScript`))