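; BP_SSlidingWall is an interactable puzzle wall that slides between its starting position and that position offset by MovingRange.
; BeginPlay caches both endpoints, and Interact drives a Timeline that lerps the actor's location between them without sweep.
; On finish the endpoints swap, so each completed slide reverses the next one.
; The PlayFromStart flag keeps interactions during a slide from restarting it.
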(event `self.ReceiveBeginPlay`
  (`parent.ReceiveBeginPlay`)
  (bind _output_get (set `self.OriginLocation` (`self.K2_GetActorLocation` self)))
  (set `self.TargetLocation` (+ (`self.MovingRange`) _output_get)))

(event `SInteractInterface.Interact`
  (if (`self.bPlayFromStart`)
    (bind (_direction _alpha) (`Timeline|Timeline` :!via `PlayFromStart` :!label _label)
      (:`Update`
        (set `self.bPlayFromStart` false)
        (`self.K2_SetActorLocation` (`KismetMathLibrary.VLerp` (`self.OriginLocation`) (`self.TargetLocation`) _alpha)))
      (:`Finished`
        (bind _output_get (set `self.Temp` (`self.OriginLocation`)))
        (set `self.OriginLocation` (`self.TargetLocation`))
        (set `self.TargetLocation` _output_get)
        (set `self.bPlayFromStart` true)))
    (else
      (goto _label))))

(fn `UserConstructionScript`
  (`parent.UserConstructionScript`))