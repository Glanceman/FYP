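; BP_SRotatingWall is an interactable puzzle wall that rotates about its Pivot between its starting yaw and that yaw plus MovingRange.
; Interact spawns a looping stone-scrape sound if none is active and runs a Timeline that lerps the pivot's yaw.
; On finish it stops the sound and swaps origin and target, so the next interaction reverses the turn.
; A PlayFromStart flag keeps interactions mid-turn from restarting the Timeline.
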(event `self.ReceiveBeginPlay`
  (bind (_relativerotation_roll _relativerotation_pitch _relativerotation_yaw) (`KismetMathLibrary.BreakRotator` (`SceneComponent.RelativeRotation` (`self.Pivot`))))
  (`parent.ReceiveBeginPlay`)
  (bind _output_get (set `self.OriginYaw` _relativerotation_yaw))
  (set `self.TargetYaw` (+ (`self.MovingRange`) _output_get)))

(event `SInteractInterface.Interact`
  (bind _audiocomponent (`self.AudioComponent`))
  (`/Engine/EditorBlueprintResources/StandardMacros.IsValid` _audiocomponent
    (:`Is Valid`
      (if (`ActorComponent.IsBeingDestroyed` _audiocomponent)
        (bind _returnvalue (`GameplayStatics.SpawnSoundAtLocation` "/Game/FYP_Content/BP/Actor/Door/Sound/StoneScrapeLoop_Cue.StoneScrapeLoop_Cue" (`self.K2_GetActorLocation`) (struct) 1.0 1.0 0.0 null null :!label _label))
        (set `self.AudioComponent` _returnvalue)))
    (:`Is Not Valid`
      (goto _label)))
  (if (`self.bPlayFromStart`)
    (bind (_direction _alpha) (`Timeline|Timeline` :!via `PlayFromStart` :!label _label_2)
      (:`Update`
        (set `self.bPlayFromStart` false)
        (`SceneComponent.K2_SetRelativeRotation` (`self.Pivot`) (`KismetMathLibrary.MakeRotator` 0.0 0.0 (`KismetMathLibrary.Lerp` (`self.OriginYaw`) (`self.TargetYaw`) _alpha)) false false))
      (:`Finished`
        (bind _output_get (set `self.Temp` (`self.OriginYaw`)))
        (set `self.OriginYaw` (`self.TargetYaw`))
        (set `self.TargetYaw` _output_get)
        (`AudioComponent.Stop` (`self.AudioComponent`))
        (set `self.bPlayFromStart` true)))
    (else
      (goto _label_2))))

(fn `UserConstructionScript`
  (`parent.UserConstructionScript`))