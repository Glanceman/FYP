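; Base actor for interactive puzzle walls that shows a widget and offers itself as the character's interaction target on overlap.
; The construction script fits an axis-aligned Box around the Wall bounds with padding, and BeginPlay moves the Widget to the actor's bounds center.
; Any actor overlap toggles the Widget, while BP_SCharacter also has InteractObject set on entry and cleared on exit.
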(event `self.ReceiveBeginPlay`
  (`SceneComponent.K2_SetWorldLocation` (`self.Widget`) (`self.GetActorBounds` false) false false))

(event `self.ReceiveActorBeginOverlap`
  (params (OtherActor :type "Actor Object Reference"))
  (`SceneComponent.SetHiddenInGame` (`self.Widget`) false false)
  (bind _asbp_scharacter (cast `/Game/FYP_Content/BP/Character/Hero/BP_SCharacter` OtherActor))
  (set `/Game/FYP_Content/BP/Character/Hero/BP_SCharacter.InteractObject` self _asbp_scharacter))

(event `self.ReceiveActorEndOverlap`
  (params (OtherActor :type "Actor Object Reference"))
  (`SceneComponent.SetHiddenInGame` (`self.Widget`) true false)
  (bind _asbp_scharacter (cast `/Game/FYP_Content/BP/Character/Hero/BP_SCharacter` OtherActor))
  (set `/Game/FYP_Content/BP/Character/Hero/BP_SCharacter.InteractObject` null _asbp_scharacter))

(fn `UserConstructionScript`
  (bind _box (`self.Box`))
  (bind (_origin _boxextent) (`KismetSystemLibrary.GetComponentBounds` (`self.Wall`)))
  (`SceneComponent.K2_SetWorldLocation` _box _origin false false)
  (`BoxComponent.SetBoxExtent` _box (+ _boxextent 50.0) false)
  (`SceneComponent.SetWorldScale3D` _box (1.0 1.0 1.0))
  (`SceneComponent.K2_SetWorldRotation` :`self` _box))