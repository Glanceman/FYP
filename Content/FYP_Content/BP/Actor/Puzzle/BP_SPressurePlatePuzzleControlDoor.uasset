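; A pressure plate puzzle controller, apparently for a door, that unlocks or locks its linked TriggerableActor based on the puzzle outcome.
; Succeed sends the unlock trigger message to that actor, then clears Solved back to false, while Fail sends the lock message.
; It holds no plate detection logic of its own, as BeginPlay, overlap and Tick are disabled stubs and the construction script only calls its parent.
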(event `self.Succeed`
  (message `SPuzzleTriggerInterface.TriggerToUnlock` (`self.TriggerableActor`))
  (set `self.bSolved` false))

(event `self.Fail`
  (message `SPuzzleTriggerInterface.TriggerToLock` (`self.TriggerableActor`)))

(fn `UserConstructionScript`
  (`parent.UserConstructionScript`))