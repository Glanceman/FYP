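; BP_SPressurePlatePuzzle2 is a puzzle manager that is solved when all of its pressure plates are on at the same time.
; On BeginPlay it registers itself as each plate's parent and turns off their trigger-only-on-enter mode.
; Plate notifications adjust a running count of active plates.
; When the count matches the total, it unlocks the assigned TriggerableActor through SPuzzleTriggerInterface and marks itself solved.
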(event `self.ReceiveBeginPlay`
  (bind _plates (`self.Plates`))
  (for _array_element _plates
    (`SPressurePlate.SetParentLater` _array_element self)
    (set `SPressurePlate.bOnlyTriggerByEnter` false _array_element)
    (set `self.NumberOfPlates` (`KismetArrayLibrary.Array_Length` (`self.Plates`))))
  (`KismetSystemLibrary.PrintString` "Set Parent Complete")
  (`KismetSystemLibrary.PrintString` (`KismetStringLibrary.Conv_IntToString` (`KismetArrayLibrary.Array_Length` _plates))))

(event `self.NotifyFromChildActor`
  (params (Child :type "Actor Object Reference"))
  (`KismetSystemLibrary.PrintString` "Notify")
  (`|ExecutionSequence`
    (:`then_0`
      (bind _asbp_spressure_plate (cast `/Game/FYP_Content/BP/Actor/Puzzle/BP_SPressurePlate` Child))
      (if (== (`SPressurePlate.bOn` _asbp_spressure_plate) true)
        (set `self.NumberOfOnPlates` (+ (`self.NumberOfOnPlates`) 1))
        (else
          (set `self.NumberOfOnPlates` (- (`self.NumberOfOnPlates`) 1)))))
    (:`then_1`
      (if (== (`self.NumberOfOnPlates`) (`self.NumberOfPlates`))
        (`KismetSystemLibrary.PrintString` "Solved")
        (`self.Succeed`)))))

(event `self.Succeed`
  (bind _triggerableactor (`self.TriggerableActor`))
  (`/Engine/EditorBlueprintResources/StandardMacros.IsValid` _triggerableactor
    (:`Is Valid`
      (if (`KismetSystemLibrary.DoesImplementInterface` _triggerableactor "/Script/FYP.SPuzzleTriggerInterface")
        (message `SPuzzleTriggerInterface.TriggerToUnlock` _triggerableactor)
        (set `self.bSolved` true)))
    (:`Is Not Valid`
      (`KismetSystemLibrary.PrintString` "Triggerable Actor not set yet"))))

(fn `UserConstructionScript`
  (`parent.UserConstructionScript`))