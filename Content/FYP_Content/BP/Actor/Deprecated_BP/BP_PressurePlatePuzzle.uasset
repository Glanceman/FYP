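; Pressure plate puzzle actor that is solved if every plate counts as pressed when the player character leaves the puzzle area.
; The construction script spawns a Rows-by-Cols grid of child actors, counts them and fits a Box around their bounds.
; On end overlap, a full pressed count marks it solved, otherwise a short delay precedes zeroing the count and resetting each BP_PressurePlate.
; The pressed count is never incremented here.
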(event `self.ReceiveBeginPlay`
  (`KismetSystemLibrary.PrintString` (`KismetStringLibrary.Conv_IntToString` (`KismetArrayLibrary.Array_Length` (`self.GetAllChildActors` false)))))

(event `self.ReceiveActorEndOverlap`
  (params (OtherActor :type "Actor Object Reference"))
  (if (== (`self.bSolved`) false)
    (cast `SCharacter` OtherActor)
    (if (== (`self.NumberOfPressed`) (`self.NumberOfPlates`))
      (`self.Succeed`)
      (else
        (`self.Fail`)))))

(event `Succeed`
  (set `self.bSolved` true)
  (`KismetSystemLibrary.PrintString` "Solved"))

(event `Fail`
  (`KismetSystemLibrary.Delay` 0.2)
  (set `self.NumberOfPressed` 0)
  (for _array_element (`self.GetAllChildActors` true)
    (bind _asbp_pressure_plate (cast `/Game/FYP_Content/BP/Actor/Deprecated_BP/BP_PressurePlate` _array_element))
    (`/Game/FYP_Content/BP/Actor/Deprecated_BP/BP_PressurePlate.Reset` _asbp_pressure_plate)))

(fn `UserConstructionScript`
  (bind _childactors (`self.GetAllChildActors` false))
  (bind _spacing (`self.Spacing`))
  (bind _box (`self.Box`))
  (`|ExecutionSequence`
    (:`then_0`
      (for _index (range (`self.Rows`))
        (for _index_2 (range (`self.Cols`))
          (`AddComponent|NODE_AddChildActorComponent-0` :`RelativeTransform` (`KismetMathLibrary.MakeTransform` (`KismetMathLibrary.MakeVector` (`KismetMathLibrary.Conv_IntToDouble` (* _spacing _index_2)) (`KismetMathLibrary.Conv_IntToDouble` (* _spacing _index))))))))
    (:`then_1`
      (set `self.NumberOfPlates` (`KismetArrayLibrary.Array_Length` _childactors))
      (bind (_center _boxextent) (`GameplayStatics.GetActorArrayBounds` _childactors true))
      (`BoxComponent.SetBoxExtent` _box (`KismetMathLibrary.MakeVector` (.x _boxextent) (.y _boxextent) 100.0) true)
      (`SceneComponent.K2_SetWorldLocation` _box _center false false))))