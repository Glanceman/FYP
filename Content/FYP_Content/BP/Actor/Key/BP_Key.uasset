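; BP_Key is a key actor that can start hidden in the game and be revealed by a trigger event.
; On BeginPlay, if HiddenInGame is set, it hides the static mesh with its children and disables the box collision.
; TriggertoUnlock shows the mesh again, restores query-only collision on the box and prints a debug string.
; The graph holds no pickup logic.
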(event `self.ReceiveBeginPlay`
  (if (`self.HiddenInGame`)
    (`SceneComponent.SetHiddenInGame` (`self.StaticMesh`) true true)
    (`PrimitiveComponent.SetCollisionEnabled` (`self.Box`) "NoCollision")))

(event `SPuzzleTriggerInterface.TriggerToUnlock`
  (`KismetSystemLibrary.PrintString` "Trigger")
  (`SceneComponent.SetHiddenInGame` (`self.StaticMesh`) false true)
  (`PrimitiveComponent.SetCollisionEnabled` (`self.Box`) "QueryOnly"))

(fn `UserConstructionScript`
  (`parent.UserConstructionScript`))