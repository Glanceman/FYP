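; Anim notify state that opens a body-component hit detection window during skeleton enemy animations.
; On begin it casts the mesh owner to BP_Skeleton_Enemy and calls StartBodyComponentTrack with its ComponentName.
; On end it calls StopHitDetection on the same enemy.
; A failed cast in either event only prints a debug string, so it works only on that enemy class.
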(fn `Received_NotifyBegin`
  (params (MeshComp :type "SkeletalMeshComponent Object Reference") (Animation :type "AnimSequenceBase Object Reference") (TotalDuration :type "Float (single-precision)") (EventReference :type "AnimNotifyEventReference Structure (by ref)"))
  (returns (ReturnValue :type Boolean))
  (bind _asbp_skeleton_enemy (cast `/Game/FYP_Content/BP/Character/SkeletonEnemy/Blueprint/BP_Skeleton_Enemy` (`ActorComponent.GetOwner` MeshComp))
    (:`then`
      (`/Game/FYP_Content/BP/Character/SkeletonEnemy/Blueprint/BP_Skeleton_Enemy.BP_StartBodyComponentTrack` _asbp_skeleton_enemy (`self.ComponentName`)))
    (:`CastFailed`
      (`KismetSystemLibrary.PrintString` null "Fail Cast to Enemy in BodyComponentState")))
  (return true))

(fn `Received_NotifyEnd`
  (params (MeshComp :type "SkeletalMeshComponent Object Reference") (Animation :type "AnimSequenceBase Object Reference") (EventReference :type "AnimNotifyEventReference Structure (by ref)"))
  (returns (ReturnValue :type Boolean))
  (bind _asbp_skeleton_enemy (cast `/Game/FYP_Content/BP/Character/SkeletonEnemy/Blueprint/BP_Skeleton_Enemy` (`ActorComponent.GetOwner` MeshComp))
    (:`then`
      (`/Game/FYP_Content/BP/Character/SkeletonEnemy/Blueprint/BP_Skeleton_Enemy.BP_StopHitDetection` _asbp_skeleton_enemy))
    (:`CastFailed`
      (`KismetSystemLibrary.PrintString` null "End: Fail Cast to Enemy in BodyComponentState")))
  (return true))