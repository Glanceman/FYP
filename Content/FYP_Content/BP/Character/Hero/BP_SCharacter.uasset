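; Player hero Blueprint with katana melee plus a throwable blade that can be recalled or teleported to.
; Holding Throw/Teleport eases the camera into aim; release plays the throw montage or teleports to the thrown blade, shoving whatever it hit.
; Throw spawns the projectile along a camera-traced direction and hides the katana until teleport or catch.
; Also handles hit-detection toggles, directional hit reactions, death and per-tick debug arrows; older attack logic remains unconnected.
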(event `self.ReceiveBeginPlay`
  (bind _asabp_scharacter (cast `/Game/FYP_Content/BP/Character/Hero/ABP_SCharacter` (`SkeletalMeshComponent.GetAnimInstance` (`self.Mesh`))))
  (set `self.AimRef` _asabp_scharacter))

(event `self.ReceiveTick`
  (params (DeltaSeconds :type "Float (single-precision)"))
  (`|ExecutionSequence`
    (:`then_0`
      (`self.DrawDebugArrows`)
      (`/Engine/EditorBlueprintResources/StandardMacros.IsValid` (`self.BP_Weapon`)
        (:`Is Not Valid`
          (bind _asbp_skatana_base (cast `/Game/FYP_Content/BP/Weapon/BP_SKatanaBase` (`self.GetWeapon`)))
          (set `self.BP_Weapon` _asbp_skatana_base))))))

(event `BP_EndHitDetection`
  ;[1 1 1] Attack/End Attack
  (set `self.bAttack` false)
  (`SKatanaBase.StopDetectionEvent` (`self.BP_Weapon`)))

(event `BP_StartHitDetection`
  ;[1 1 1] Attack/End Attack
  (`SKatanaBase.AttackDetectionEvent` (`self.BP_Weapon`)))

(event `InputAction|Throw/Teleport`
  (params (Key :type "Key Structure"))
  (bind _camera (`self.Camera`))
  (bind _returnvalue (`self.GetAttachParentActor` (`self.ThownWeapon`)))
  (bind _returnvalue_2 (`SkeletalMeshComponent.GetAnimInstance` (`self.Mesh`)))
  (bind _returnvalue_3 (`self.GetComponentByClass` _returnvalue "/Script/Engine.PrimitiveComponent"))
  ;[1 1 1] Throw
  (:`Pressed`
    (set `CharacterMovementComponent.bOrientRotationToMovement` false (`self.CharacterMovement`))
    (set `self.bUseControllerRotationYaw` true)
    (set `/Game/FYP_Content/BP/Character/Hero/ABP_SCharacter.bAimMode` true (`self.AimRef`))
    (bind _returnvalue_4 (`|CreateWidget` "/Game/FYP_Content/BP/UI/HUD_Aim.HUD_Aim_C"))
    (bind _output_get (set `self.HUD_Aim` _returnvalue_4))
    (`UserWidget.AddToViewport` _output_get 0)
    (bind (_direction _cameraalpha) (`Timeline|AimTimeLine` :!via `PlayFromStart` :!label _label)
      (:`Update`
        (`SceneComponent.K2_SetRelativeLocation` _camera (`KismetMathLibrary.VLerp` (0.0 0.0 0.0) (200.0 30.0 30.0) _cameraalpha) false false)
        (`CameraComponent.SetFieldOfView` _camera (`KismetMathLibrary.Lerp` 90.0 75.0 _cameraalpha)))))
  (:`Released`
    (`|ExecutionSequence`
      (:`then_0`
        (set `CharacterMovementComponent.bOrientRotationToMovement` true (`self.CharacterMovement`))
        (set `self.bUseControllerRotationYaw` false)
        (set `/Game/FYP_Content/BP/Character/Hero/ABP_SCharacter.bAimMode` false (`self.AimRef`))
        (`Widget.RemoveFromParent` (`self.HUD_Aim`))
        (goto _label :!via `Reverse`))
      (:`then_1`
        (`/Engine/EditorBlueprintResources/StandardMacros.IsValid` (`self.ThownWeapon`)
          (:`Is Valid`
            (`self.K2_SetActorLocation` (`self.K2_GetActorLocation` (`self.ThownWeapon`)) false true)
            (`|ExecutionSequence`
              (:`then_0`
                (bind _ascharacter (cast `Character` _returnvalue)
                  (:`then`
                    (`self.LaunchCharacter` _ascharacter (+ (* (`self.GetActorForwardVector` self) 1000) (0.0 0.0 100.0)) false false))
                  (:`CastFailed`
                    (if (`KismetSystemLibrary.IsValid` _returnvalue)
                      (if (and (`KismetSystemLibrary.IsValid` _returnvalue_3) (`SceneComponent.IsSimulatingPhysics` _returnvalue_3 "None"))
                        (`PrimitiveComponent.AddImpulse` _returnvalue_3 (* (`self.GetActorForwardVector` self) 1000) "None" true))))))
              (:`then_1`
                (`self.K2_DestroyActor` (`self.ThownWeapon`))
                (`SceneComponent.SetVisibility` (`SKatanaBase.Katana` (`self.BP_Weapon`)) true false)
                (set `self.bWeaponOnHand` true))
              (:`then_2`
                (`AnimInstance.Montage_Stop` _returnvalue_2 0.0 (`AnimInstance.GetCurrentActiveMontage` _returnvalue_2)))))
          (:`Is Not Valid`
            (`KismetSystemLibrary.PrintString` "Throw")
            (`self.PlayAnimMontage` "/Game/FYP_Content/Animation/Retargeted/Equip_Weapon/AM_WeaponThrow.AM_WeaponThrow")))))))

(event `InputAction|Attack`
  (params (Key :type "Key Structure"))
  ;[1 1 1] Attack/End Attack
  (:`Pressed`
    (if (and (`self.bWeaponOnHand`) (`self.bIsAttachWeapon`) (== (`self.bAttack`) false))
      (`SAttackInterface.BasicAttack`))))

(event `InputAction|Pull`
  (params (Key :type "Key Structure"))
  ;[1 1 1] Recall events
  (:`Pressed`
    (if (and (not (`self.bWeaponOnHand`)) (`KismetSystemLibrary.IsValid` (`self.ThownWeapon`)))
      (`self.PlayAnimMontage` "/Game/FYP_Content/Animation/Retargeted/Equip_Weapon/AM_Weapon_Catching.AM_Weapon_Catching")
      (bind _asbp_sblade_base (cast `/Game/FYP_Content/BP/Weapon/BP_SBladeBase` (`self.ThownWeapon`)))
      (`/Game/FYP_Content/BP/Weapon/BP_SBladeBase.Recall_Event` _asbp_sblade_base))))

(event `self.ReceiveAnyDamage`
  (params (Damage :type "Float (single-precision)") (DamageType :type "DamageType Object Reference") (InstigatedBy :type "Controller Object Reference") (DamageCauser :type "Actor Object Reference"))
  (bind _attributecomponent (`self.AttributeComponent`))
  (bind _mesh (`self.Mesh`))
  (bind _returnvalue (`SkeletalMeshComponent.GetAnimInstance` _mesh))
  (`SAttributeComponent.ApplyHealthChange` _attributecomponent (* Damage -1.0))
  (if (> (`SAttributeComponent.Health` _attributecomponent) 0.0)
    (`|ExecutionSequence`
      (:`then_0`
        ;[1 1 1] handle hit animation
        (bind _returnvalue_2 (`SMathLibrary.SignedAngleBetweenTwoVectors` (`self.GetActorForwardVector` DamageCauser) (`self.GetActorForwardVector`)))
        (`|ExecutionSequence`
          (:`then_0`
            (bind _returnvalue_3 (`KismetMathLibrary.Abs` _returnvalue_2))
            (if (< _returnvalue_3 45.0)
              (set `self.Direction` "B")
              (elif (`KismetMathLibrary.InRange_FloatFloat` _returnvalue_3 45.0 135.0 true false)
                (if (== (`KismetMathLibrary.SignOfFloat` _returnvalue_2) 1.0)
                  (set `self.Direction` "R")
                  (else
                    (set `self.Direction` "L")))
                (else
                  (set `self.Direction` "F")))))
          (:`then_1`
            (`self.PlayAnimMontage` self "/Game/FYP_Content/Animation/Retargeted/Equip_Weapon/AM_GetHit.AM_GetHit" 1.0 (`self.Direction`))
            (`KismetSystemLibrary.Delay` 1.0)
            (set `self.bAttack` false)))))
    (else
      (set `self.CharacterState` "Alive")
      (`self.DisableInput` (`GameplayStatics.GetPlayerController` 0))
      (`AIPerceptionStimuliSourceComponent.UnregisterFromPerceptionSystem` (`self.AIPerceptionStimuliSource`))
      (`|PlayMontage` _mesh "/Game/FYP_Content/Animation/Retargeted/Equip_Weapon/AM_Die.AM_Die" 1.0 0.0 "2"
        (:`OnNotifyBegin`
          (`AnimInstance.Montage_Pause` _returnvalue (`AnimInstance.GetCurrentActiveMontage` _returnvalue)))))))

(event `Caught`
  ;[1 1 1] Recall events
  (`self.PlayAnimMontage` "/Game/FYP_Content/Animation/Retargeted/Equip_Weapon/AM_Weapon_Caught.AM_Weapon_Caught")
  (`SceneComponent.SetVisibility` (`SKatanaBase.Katana` (`self.BP_Weapon`)) true false)
  (set `self.bWeaponOnHand` true)
  (`self.K2_DestroyActor` (`self.ThownWeapon`)))

(fn `BP_EquipWeapon`
  (`self.PlayAnimMontage` "/Game/FYP_Content/Animation/Retargeted/Equip_Weapon/AM_EquipWeapon_1.AM_EquipWeapon_1")
  (`self.AttachWeapon`))

(fn `BP_FindTarget`
  (params (Length :type Integer))
  (returns (Target :type "SCharacterBase Object Reference"))
  (bind _camera (`self.Camera`))
  (bind _returnvalue (`SceneComponent.K2_GetComponentLocation` _camera))
  (bind (_outhit _returnvalue_2) (`KismetSystemLibrary.SphereTraceSingle` :`Start` _returnvalue :`End` (+ _returnvalue (* (`SceneComponent.GetForwardVector` _camera) (`local.Length`))) :`Radius` 100.0 :`TraceChannel` "TraceTypeQuery1" :`DrawDebugType` "ForDuration"))
  (if _returnvalue_2
    (bind _asscharacter_base (cast `SCharacterBase` (`.HitActor` (`GameplayStatics.BreakHitResult` _outhit)))
      (:`then`
        (return _asscharacter_base))
      (:`CastFailed`
        _)))
  (return null))

(fn `DrawDebugArrows`
  (bind _returnvalue (`CharacterMovementComponent.GetLastUpdateVelocity` (`self.CharacterMovement`)))
  (bind _returnvalue_2 (- (`self.K2_GetActorLocation` self) (0.0 0.0 80.0)))
  (`|ExecutionSequence`
    (:`then_0`
      (if (> (`KismetMathLibrary.VSize` _returnvalue) 0.0)
        (`KismetSystemLibrary.DrawDebugArrow` _returnvalue_2 (+ (* _returnvalue (1.0 1.0 0.0)) _returnvalue_2) 10.0 (struct :`R` 1.0 :`A` 1.0) 0.0 1.0)))
    (:`then_1`
      (`KismetSystemLibrary.DrawDebugArrow` _returnvalue_2 (+ _returnvalue_2 (* (`KismetMathLibrary.Normal` (* (`self.GetActorForwardVector` self) (1.0 1.0 0.0))) (`KismetMathLibrary.Conv_DoubleToVector` 100.0))) 0.0 (struct :`R` 0.994245 :`G` 1.0 :`A` 1.0)))))

(fn `Throw`
  (bind (_returnvalue_roll _returnvalue_pitch _returnvalue_yaw) (`KismetMathLibrary.BreakRotator` (`self.GetControlRotation`)))
  (set `self.ShootLocation` (`SceneComponent.GetSocketLocation` (`self.Mesh`) "DEF-weapon_R"))
  (`|ExecutionSequence`
    (:`then_0`
      ;[1 1 1] Set Aiming Start/End location
      (set `self.AimStartLocation` (`SceneComponent.K2_GetComponentLocation` (`self.Camera`)))
      (set `self.AimEndLocation` (+ (* (`KismetMathLibrary.Conv_DoubleToVector` 10000.0) (`KismetMathLibrary.Normal` (`SceneComponent.GetForwardVector` (`self.Camera`)))) (`self.AimStartLocation`))))
    (:`then_1`
      ;[1 1 1] Set shooting Direction
      (bind _asactor (cast `Actor` self))
      (bind _outhit (`KismetSystemLibrary.LineTraceSingle` (`self.AimStartLocation`) (`self.AimEndLocation`) "TraceTypeQuery1" false (`|MakeArray` _asactor)))
      (bind (_bblockinghit _binitialoverlap _time _distance _location _impactpoint) (`GameplayStatics.BreakHitResult` _outhit))
      (if _bblockinghit
        (set `self.ShootDir` (`KismetMathLibrary.Normal` (- _impactpoint (`self.ShootLocation`))))
        (else
          (set `self.ShootDir` (`KismetMathLibrary.Normal` (- (`self.AimEndLocation`) (`self.AimStartLocation`)))))))
    (:`then_2`
      (bind _returnvalue (`SKatanaBase.GetProjectileClass` (`self.BP_Weapon`)))
      (bind _returnvalue_2 (`|SpawnActorFromClass` _returnvalue (`KismetMathLibrary.MakeTransform` (`self.ShootLocation`) (`KismetMathLibrary.MakeRotator` _returnvalue_roll 0.0 _returnvalue_yaw)) "Undefined" "OverrideRootScale" null null))
      (bind _output_get (set `self.ThownWeapon` _returnvalue_2))
      (bind _asbp_sblade_base (cast `/Game/FYP_Content/BP/Weapon/BP_SBladeBase` _output_get))
      (`/Game/FYP_Content/BP/Weapon/BP_SBladeBase.ShootInDirection` _asbp_sblade_base (`self.ShootDir`))
      (`SceneComponent.SetVisibility` (`SKatanaBase.Katana` (`self.BP_Weapon`)) false false)
      (set `self.bWeaponOnHand` false))))

(fn `UserConstructionScript`)