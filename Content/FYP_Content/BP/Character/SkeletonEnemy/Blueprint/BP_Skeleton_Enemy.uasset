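; Skeleton enemy character with modular gear, a montage-driven basic attack, and health that destroys it at zero.
; The construction script links gear meshes to the body's pose and toggles each part's visibility and collision from flags.
; Incoming damage updates the AttributeComponent and plays a hit montage.
; Start/stop events run looping timer sphere traces between previous and current bone positions, damaging each hit actor once per tracking window.
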(event `self.ReceiveBeginPlay`
  (`SkeletalMeshComponent.Play` (`self.SK_Bow`) (`self.BowAnimAttackPlay`)))

(event `self.ReceiveAnyDamage`
  (params (Damage :type "Float (single-precision)") (DamageType :type "DamageType Object Reference") (InstigatedBy :type "Controller Object Reference") (DamageCauser :type "Actor Object Reference"))
  (bind _attributecomponent (`self.AttributeComponent`))
  (bind _health (`SAttributeComponent.Health` _attributecomponent))
  (`SAttributeComponent.ApplyHealthChange` _attributecomponent (* Damage -1.0))
  (`AnimInstance.Montage_Play` (`SkeletalMeshComponent.GetAnimInstance` (`self.Mesh`)) "/Game/FYP_Content/BP/Character/SkeletonEnemy/Animations/AM_Hit.AM_Hit" 1.0 "MontageLength" 0.0 true)
  (if (<= _health 0.0)
    (`self.K2_DestroyActor`)
    (`KismetSystemLibrary.PrintString` "Destroy")
    (else
      (`KismetSystemLibrary.PrintText` (`KismetTextLibrary.Conv_DoubleToText` _health "HalfToEven")))))

(event `BP_StartBodyComponentTrack`
  (params (ComponentName :type "Array of Name"))
  (set `self.TrackingBones` ComponentName)
  (`|ExecutionSequence`
    (:`then_0`
      (bind _output_get (set `self.Prev_TrackingPointsBP` (`self.BP_GetTrackingPointsFromBones` (`self.TrackingBones`) (`self.Mesh`))))
      (`KismetArrayLibrary.Array_Clear` (`self.HitActors_BP`)))
    (:`then_1`
      (bind _returnvalue (`KismetSystemLibrary.K2_SetTimerDelegate` (delegate `HitDetection`) 0.05 true))
      (set `self.TimerHandle` _returnvalue))))

(event `HitDetection`
  (bind _output_get (set `self.Cur_TrackingPointBP` (`self.BP_GetTrackingPointsFromBones` (`self.TrackingBones`) (`self.Mesh`))))
  (for (_array_element _array_index) _output_get
    (bind (_outhit _returnvalue) (`KismetSystemLibrary.SphereTraceSingle` :`Start` (`|GetArrayItem` (`self.Prev_TrackingPointsBP`) _array_index) :`End` _array_element :`Radius` 20.0 :`TraceChannel` "TraceTypeQuery1" :`DrawDebugType` "ForDuration"))
    (if _returnvalue
      (bind (_bblockinghit _binitialoverlap _time _distance _location _impactpoint _normal _impactnormal _physmat _hitactor) (`GameplayStatics.BreakHitResult` _outhit))
      (if (== (`KismetArrayLibrary.Array_Find` (`self.HitActors_BP`) _hitactor) -1)
        (`KismetSystemLibrary.PrintString` (`KismetSystemLibrary.GetDisplayName` _hitactor))
        (`GameplayStatics.ApplyDamage` _hitactor (`self.BasicDamageValue`) (`self.GetInstigatorController`) self "/Script/Engine.DamageType")
        (`KismetArrayLibrary.Array_Add` (`self.HitActors_BP`) _hitactor))))
  (set `self.Prev_TrackingPointsBP` (`self.Cur_TrackingPointBP`))
  (`KismetArrayLibrary.Array_Clear` (`self.Cur_TrackingPointBP`)))

(event `BP_StopHitDetection`
  (bind _timerhandle (`self.TimerHandle`))
  (if (`KismetSystemLibrary.K2_IsValidTimerHandle` _timerhandle)
    (`KismetSystemLibrary.K2_ClearAndInvalidateTimerHandle` _timerhandle)))

(fn `BasicAttack`
  (message `/Game/FYP_Content/BP/Interface/I_PlayMontage.PlayAttackMontage` (`SkeletalMeshComponent.GetAnimInstance` (`self.Mesh`)) (`self.AM_BasicAttack`)))

(fn `BP Turn on/ Off Component`
  (params (TargetMesh :type "PrimitiveComponent Object Reference") (bEnable :type Boolean) (bToChildren :type Boolean) (CollisionType :type "ECollisionEnabled Enum" :default "QueryOnly"))
  (if bEnable
    (`SceneComponent.SetVisibility` TargetMesh true (`local.bToChildren`))
    (`SceneComponent.SetVisibility` (`local.TargetMesh`) true (`local.bToChildren`))
    (`PrimitiveComponent.SetCollisionEnabled` TargetMesh (`local.CollisionType`))
    (`PrimitiveComponent.SetCollisionEnabled` (`local.TargetMesh`) (`local.CollisionType`))
    (if (`local.bToChildren`)
      (for _array_element (`SceneComponent.GetChildrenComponents` (`local.TargetMesh`) true)
        (bind _asprimitive_component (cast `PrimitiveComponent` _array_element))
        (`PrimitiveComponent.SetCollisionEnabled` _asprimitive_component "QueryAndPhysics")))
    (else
      (`SceneComponent.SetVisibility` TargetMesh false (`local.bToChildren`))
      (`SceneComponent.SetVisibility` (`local.TargetMesh`) false (`local.bToChildren`))
      (`PrimitiveComponent.SetCollisionEnabled` TargetMesh "NoCollision")
      (`PrimitiveComponent.SetCollisionEnabled` (`local.TargetMesh`) "NoCollision")
      (if (`local.bToChildren`)
        (for _array_element_2 (`SceneComponent.GetChildrenComponents` (`local.TargetMesh`) true)
          (bind _asprimitive_component_2 (cast `PrimitiveComponent` _array_element_2))
          (`PrimitiveComponent.SetCollisionEnabled` _asprimitive_component_2 "NoCollision"))))))

(fn `BP_GetTrackingPointsFromBones`
  (params (BoneNames :type "Array of Name") (Mesh :type "SkeletalMeshComponent Object Reference"))
  (returns (TrackingPoints :type "Array of Vector Structure"))
  (locals (TempTrackingPoints :type "Array of Vector Structure"))
  (`KismetArrayLibrary.Array_Clear` (`local.TempTrackingPoints`))
  (for _array_element BoneNames
    (`KismetArrayLibrary.Array_Add` (`local.TempTrackingPoints`) (`SceneComponent.GetSocketLocation` (`local.Mesh`) _array_element)))
  (return (`local.TempTrackingPoints`)))

(fn `UserConstructionScript`
  (`SkinnedMeshComponent.SetLeaderPoseComponent` (`self.SK_HelmetPart`) (`self.Mesh`) false false)
  (`SkinnedMeshComponent.SetLeaderPoseComponent` (`self.SK_Bandage1`) (`self.Mesh`) false false)
  (`SkinnedMeshComponent.SetLeaderPoseComponent` (`self.SK_Bandage2`) (`self.Mesh`) false false)
  (`SkinnedMeshComponent.SetLeaderPoseComponent` (`self.SK_Bandage3`) (`self.Mesh`) false false)
  (`SkinnedMeshComponent.SetLeaderPoseComponent` (`self.SK_Belt`) (`self.Mesh`) false false)
  (`SkinnedMeshComponent.SetLeaderPoseComponent` (`self.SK_Helmet`) (`self.Mesh`) false false)
  (`SkinnedMeshComponent.SetLeaderPoseComponent` (`self.SK_Armor`) (`self.Mesh`) false false)
  (`SkinnedMeshComponent.SetLeaderPoseComponent` (`self.SK_Rag1`) (`self.Mesh`) false false)
  (`SkinnedMeshComponent.SetLeaderPoseComponent` (`self.SK_Quiver`) (`self.Mesh`) false false)
  (`SkinnedMeshComponent.SetLeaderPoseComponent` (`self.SK_Rag2`) (`self.Mesh`) false false)
  (`SkinnedMeshComponent.SetLeaderPoseComponent` (`self.SK_Rag3`) (`self.Mesh`) false false)
  (`SkinnedMeshComponent.SetLeaderPoseComponent` (`self.SK_Rag4`) (`self.Mesh`) false false)
  (`SkinnedMeshComponent.SetLeaderPoseComponent` (`self.SK_Rag5`) (`self.Mesh`) false false)
  (`|ExecutionSequence`
    (:`then_0`
      (`self.BP Turn on/ Off Component` (`self.SK_Armor`) (`self.ArmorVisibility`)))
    (:`then_1`
      (`self.BP Turn on/ Off Component` (`self.SK_Bandage1`) (`self.Bandage1Visibility`)))
    (:`then_2`
      (`self.BP Turn on/ Off Component` (`self.SK_Bandage2`) (`self.Bandage2Visibility`)))
    (:`then_3`
      (`self.BP Turn on/ Off Component` (`self.SK_Bandage3`) (`self.Bandage3Visibility`)))
    (:`then_4`
      (`self.BP Turn on/ Off Component` (`self.SK_Belt`) (`self.BeltVisibility`)))
    (:`then_5`
      (`self.BP Turn on/ Off Component` (`self.SK_Helmet`) (`self.HelmetVisibility`)))
    (:`then_6`
      (`self.BP Turn on/ Off Component` (`self.SK_HelmetPart`) (`self.HelmetPartVisibility`)))
    (:`then_7`
      (`self.BP Turn on/ Off Component` (`self.SK_Quiver`) (`self.QuiverVisibility`)))
    (:`then_8`
      (`self.BP Turn on/ Off Component` (`self.SK_Rag1`) (`self.Rag1Visibility`)))
    (:`then_9`
      (`self.BP Turn on/ Off Component` (`self.SK_Rag2`) (`self.Rag2Visibility`)))
    (:`then_10`
      (`self.BP Turn on/ Off Component` (`self.SK_Rag3`) (`self.Rag3Visibility`)))
    (:`then_11`
      (`self.BP Turn on/ Off Component` (`self.SK_Rag4`) (`self.Rag4Visibility`)))
    (:`then_12`
      (`self.BP Turn on/ Off Component` (`self.SK_Rag5`) (`self.Rag5Visibility`)))
    (:`then_13`
      (`self.BP Turn on/ Off Component` (`self.ParticleSystem`) (`self.FXVisibility`)))
    (:`then_14`
      (`self.BP Turn on/ Off Component` (`self.SM_ArrowCut`) (`self.ArrowsVisibility`) true))
    (:`then_15`
      (`self.BP Turn on/ Off Component` (`self.SM_Sword`) (`self.SwordVisibility`)))
    (:`then_16`
      (`self.BP Turn on/ Off Component` (`self.SK_Bow`) (`self.BowVisibility`) true))))