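; Player character Blueprint for katana combat with a throwable blade that can be recalled or teleported to.
; Attack input and Tick send montage play and end messages to the AnimInstance.
; Holding Throw/Teleport enters a timeline-blended aim camera with HUD; releasing teleports to an existing thrown blade or plays the throw montage.
; Throw traces from the camera to aim a projectile spawned at the hand socket and hides the held katana.
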(event `self.ReceiveBeginPlay`
  (bind _asabp_scharacter (cast `/Game/FYP_Content/BP/Character/ABP_SCharacter` (`SkeletalMeshComponent.GetAnimInstance` (`self.Mesh`))))
  (set `self.AimRef` _asabp_scharacter))

(event `self.ReceiveTick`
  (params (DeltaSeconds :type "Float (single-precision)"))
  (`|ExecutionSequence`
    (:`then_0`
      (`self.DrawDebugArrows`)
      (`/Engine/EditorBlueprintResources/StandardMacros.IsValid` (`self.BP_Weapon`)
        (:`Is Not Valid`
          (bind _asbp_skatana_base (cast `/Game/FYP_Content/BP/Weapon/BP_SKatanaBase` (`self.GetWeapon`)))
          (set `self.BP_Weapon` _asbp_skatana_base))))
    (:`then_1`
      (message `/Game/FYP_Content/BP/Interface/I_PlayMontage.EndAttackMontage` (`SkeletalMeshComponent.GetAnimInstance` (`self.Mesh`)) (and (not (`self.bAttack`)) (!= (`KismetMathLibrary.VSize` (`CharacterMovementComponent.GetCurrentAcceleration` (`self.CharacterMovement`))) 0.0)) (`/Game/FYP_Content/BP/Weapon/BP_SKatanaBase.AttackMontage` (`self.BP_Weapon`))))))

(event `InputAction|Attack`
  (params (Key :type "Key Structure"))
  (:`Pressed`
    (set `self.bAttack` true)
    (message `/Game/FYP_Content/BP/Interface/I_PlayMontage.PlayAttackMontage` (`SkeletalMeshComponent.GetAnimInstance` (`self.Mesh`)) (`/Game/FYP_Content/BP/Weapon/BP_SKatanaBase.AttackMontage` (`self.BP_Weapon`)))))

(event `Key|Z`
  (params (Key :type "Key Structure")))

(event `InputAction|Pull`
  (params (Key :type "Key Structure"))
  (:`Pressed`
    (if (and (not (`self.bWeaponOnHand`)) (`KismetSystemLibrary.IsValid` (`self.ThownWeapon`)))
      (bind _asbp_sblade_base (cast `/Game/FYP_Content/BP/Weapon/BP_SBladeBase` (`self.ThownWeapon`)))
      (`self.K2_DetachFromActor` (`self.ThownWeapon`) "KeepWorld" "KeepWorld" "KeepWorld")
      (`/Game/FYP_Content/BP/Weapon/BP_SBladeBase.Recall_Event` _asbp_sblade_base))))

(event `InputAction|Throw/Teleport`
  (params (Key :type "Key Structure"))
  (bind _camera (`self.Camera`))
  ;[1 1 1] Throw
  (:`Pressed`
    (set `CharacterMovementComponent.bOrientRotationToMovement` false (`self.CharacterMovement`))
    (set `self.bUseControllerRotationYaw` true)
    (set `/Game/FYP_Content/BP/Character/ABP_SCharacter.bAimMode` true (`self.AimRef`))
    (bind _returnvalue (`|CreateWidget` "/Game/FYP_Content/BP/UI/HUD_Aim.HUD_Aim_C"))
    (bind _output_get (set `self.HUD_Aim` _returnvalue))
    (`UserWidget.AddToViewport` _output_get 0)
    (bind (_direction _cameraalpha) (`Timeline|AimTimeLine` :!via `PlayFromStart` :!label _label)
      (:`Update`
        (`SceneComponent.K2_SetRelativeLocation` _camera (`KismetMathLibrary.VLerp` (0.0 0.0 0.0) (200.0 30.0 30.0) _cameraalpha) false false)
        (`CameraComponent.SetFieldOfView` _camera (`KismetMathLibrary.Lerp` 90.0 75.0 _cameraalpha)))))
  (:`Released`
    (`|ExecutionSequence`
      (:`then_0`
        (set `CharacterMovementComponent.bOrientRotationToMovement` true (`self.CharacterMovement`))
        (set `self.bUseControllerRotationYaw` false)
        (set `/Game/FYP_Content/BP/Character/ABP_SCharacter.bAimMode` false (`self.AimRef`))
        (`Widget.RemoveFromParent` (`self.HUD_Aim`))
        (goto _label :!via `Reverse`))
      (:`then_1`
        (`/Engine/EditorBlueprintResources/StandardMacros.IsValid` (`self.ThownWeapon`)
          (:`Is Valid`
            (`self.K2_SetActorLocation` (`self.K2_GetActorLocation` (`self.ThownWeapon`)) false true)
            (`self.K2_DestroyActor` (`self.ThownWeapon`))
            (`SceneComponent.SetVisibility` (`SKatanaBase.Katana` (`self.BP_Weapon`)) true false)
            (set `self.bWeaponOnHand` true))
          (:`Is Not Valid`
            (`KismetSystemLibrary.PrintString` "Throw")
            (`self.PlayAnimMontage` "/Game/FYP_Content/Animation/Retargeted/Equip_Weapon/AM_WeaponThrow.AM_WeaponThrow")))))))

(fn `BP_EquipWeapon`
  (`self.PlayAnimMontage` "/Game/FYP_Content/Animation/Retargeted/Equip_Weapon/AM_EquipWeapon_1.AM_EquipWeapon_1")
  (`self.AttachWeapon`))

(fn `DrawDebugArrows`
  (bind _returnvalue (`CharacterMovementComponent.GetLastUpdateVelocity` (`self.CharacterMovement`)))
  (bind _returnvalue_2 (- (`self.K2_GetActorLocation` self) (0.0 0.0 80.0)))
  (`|ExecutionSequence`
    (:`then_0`
      (if (> (`KismetMathLibrary.VSize` _returnvalue) 0.0)
        (`KismetSystemLibrary.DrawDebugArrow` _returnvalue_2 (+ (* _returnvalue (1.0 1.0 0.0)) _returnvalue_2) 10.0 (struct :`R` 1.0 :`A` 1.0) 0.0 1.0)))
    (:`then_1`
      (`KismetSystemLibrary.DrawDebugArrow` _returnvalue_2 (+ _returnvalue_2 (* (`KismetMathLibrary.Normal` (* (`self.GetActorForwardVector` (`self.GetController` self)) (1.0 1.0 0.0))) (`KismetMathLibrary.Conv_DoubleToVector` 100.0))) 0.0 (struct :`R` 0.994245 :`G` 1.0 :`A` 1.0)))))

(fn `Throw`
  (bind (_returnvalue_roll _returnvalue_pitch _returnvalue_yaw) (`KismetMathLibrary.BreakRotator` (`self.GetControlRotation`)))
  (set `self.ShootLocation` (`SceneComponent.GetSocketLocation` (`self.Mesh`) "DEF-weapon_R"))
  (`|ExecutionSequence`
    (:`then_0`
      ;[1 1 1] Set Aiming Start/End location
      (set `self.AimStartLocation` (`SceneComponent.K2_GetComponentLocation` (`self.Camera`)))
      (set `self.AimEndLocation` (+ (* (`KismetMathLibrary.Conv_DoubleToVector` 10000.0) (`KismetMathLibrary.Normal` (`SceneComponent.GetForwardVector` (`self.Camera`)))) (`self.AimStartLocation`))))
    (:`then_1`
      ;[1 1 1] Set shooting Direction
      (bind _asactor (cast `Actor` self))
      (bind _outhit (`KismetSystemLibrary.LineTraceSingle` (`self.AimStartLocation`) (`self.AimEndLocation`) "TraceTypeQuery1" false (`|MakeArray` _asactor)))
      (bind (_bblockinghit _binitialoverlap _time _distance _location _impactpoint) (`GameplayStatics.BreakHitResult` _outhit))
      (if _bblockinghit
        (set `self.ShootDir` (`KismetMathLibrary.Normal` (- _impactpoint (`self.ShootLocation`))))
        (else
          (set `self.ShootDir` (`KismetMathLibrary.Normal` (- (`self.AimEndLocation`) (`self.AimStartLocation`)))))))
    (:`then_2`
      (bind _returnvalue (`SKatanaBase.GetProjectileClass` (`self.BP_Weapon`)))
      (bind _returnvalue_2 (`|SpawnActorFromClass` _returnvalue (`KismetMathLibrary.MakeTransform` (`self.ShootLocation`) (`KismetMathLibrary.MakeRotator` _returnvalue_roll 0.0 (+ _returnvalue_yaw -90.0))) "Undefined" "OverrideRootScale" null null))
      (bind _output_get (set `self.ThownWeapon` _returnvalue_2))
      (bind _asbp_sblade_base (cast `/Game/FYP_Content/BP/Weapon/BP_SBladeBase` _output_get))
      (`/Game/FYP_Content/BP/Weapon/BP_SBladeBase.ShootInDirection` _asbp_sblade_base (`self.ShootDir`))
      (`SceneComponent.SetVisibility` (`SKatanaBase.Katana` (`self.BP_Weapon`)) false false)
      (set `self.bWeaponOnHand` false))))

(fn `UserConstructionScript`)